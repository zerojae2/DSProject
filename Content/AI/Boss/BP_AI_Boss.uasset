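; Boss character Blueprint that reports its health to its AI controller and handles the win sequence when it dies.
; Each Tick copies current and max health from its stats component to BP_AI_Controller_Boss.
; At zero health, a one-shot End flag gates disabling player input, playing the boss death Level Sequence and adding the win widget to the viewport.
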(event `self.ReceiveTick`
  (params (DeltaSeconds :type "Float (single-precision)"))
  (bind _bp_palyerstats (`self.BP_PalyerStats`))
  (`parent.ReceiveTick` DeltaSeconds)
  (bind _asbp_aicontroller_boss (cast `/Game/AI/Boss/BP_AIController_Boss` (`AIBlueprintHelperLibrary.GetAIController` self)))
  (set `/Game/AI/Boss/BP_AIController_Boss.health` (`/Game/Blueprints/BP_PalyerStats.Current Health` _bp_palyerstats) _asbp_aicontroller_boss)
  (set `/Game/AI/Boss/BP_AIController_Boss.maxHealth` (`/Game/Blueprints/BP_PalyerStats.Max Health` _bp_palyerstats) _asbp_aicontroller_boss)
  (if (and (== (`/Game/Blueprints/BP_PalyerStats.Current Health` (`self.BP_PalyerStats`)) 0.0) (`self.End`))
    (`self.DisableInput` (`self.player controller`))
    (bind _outactor (`LevelSequencePlayer.CreateLevelSequencePlayer` "/Game/BossDeathSequence.BossDeathSequence"))
    (`MovieSceneSequencePlayer.Play` (`LevelSequenceActor.SequencePlayer` _outactor))
    (bind _returnvalue (`|CreateWidget` "/Game/UI/WB_Win.WB_Win_C"))
    (`UserWidget.AddToViewport` _returnvalue 0)
    (set `self.End` false)))

(fn `UserConstructionScript`
  (`parent.UserConstructionScript`))