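; BP_Dummy is a damageable dummy character with a floating health bar that turns to face the player camera every tick.
; Damage plays a random hit montage and pitched sound, launches it along the player's facing, and passes to the BPPalyerStats health logic.
; When that returns true, the mesh ragdolls, a death sound plays and the bar hides.
; A separate Ragdoll event triggers delayed physics and sound.
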(event `self.ReceiveBeginPlay`
  (bind _aswb_dummy_health (cast `/Game/UI/WB_DummyHealth` (`WidgetComponent.GetWidget` (`self.Health Bar Widget`))))
  (set `self.HealthBar UI` _aswb_dummy_health))

(event `self.ReceiveTick`
  (params (DeltaSeconds :type "Float (single-precision)"))
  (`SceneComponent.K2_SetWorldRotation` (`self.Health Bar Widget`) (`KismetMathLibrary.FindLookAtRotation` (`SceneComponent.K2_GetComponentLocation` (`self.Health Bar Widget`)) (`SceneComponent.K2_GetComponentLocation` (`PlayerCameraManager.TransformComponent` (`GameplayStatics.GetPlayerCameraManager` 0)))) false false))

(event `Ragdoll`
  (`|ExecutionSequence`
    (:`then_0`
      (`KismetSystemLibrary.Delay` 2.5)
      (`PrimitiveComponent.SetSimulatePhysics` (`self.Mesh`) true))
    (:`then_1`
      (`KismetSystemLibrary.Delay` 1.7)
      (`GameplayStatics.PlaySoundAtLocation` "/Game/Audio/Deaths/Deaths.Deaths" (`self.K2_GetActorLocation`) (struct) 1.0 1.0 0.0 null null null null))))

(event `self.ReceiveAnyDamage`
  (params (Damage :type "Float (single-precision)") (DamageType :type "DamageType Object Reference") (InstigatedBy :type "Controller Object Reference") (DamageCauser :type "Actor Object Reference"))
  (`self.PlayAnimMontage` (`|GetArrayItem` (`self.hitAnims`) (`KismetMathLibrary.RandomIntegerInRange` 0 (- (`KismetArrayLibrary.Array_Length` (`self.hitAnims`)) 1))))
  (bind _asbp_third_person_character (cast `/Game/ThirdPerson/Blueprints/BP_ThirdPersonCharacter` (`GameplayStatics.GetPlayerCharacter` 0)))
  (`self.LaunchCharacter` (* (`KismetMathLibrary.GetForwardVector` (`self.K2_GetActorRotation` _asbp_third_person_character)) 700))
  (`GameplayStatics.PlaySoundAtLocation` "/Game/Audio/Deaths/Deaths.Deaths" (`self.K2_GetActorLocation`) (struct) 1.0 (`KismetMathLibrary.RandomFloatInRange` 1.5 1.3) 0.0 "/Game/Audio/SA_Character.SA_Character" null null null)
  (bind _isplayer_dead_ (`/Game/Blueprints/BP_PalyerStats.Decrease Health` (`self.BP_PalyerStats`) Damage))
  (if _isplayer_dead_
    (`PrimitiveComponent.SetSimulatePhysics` (`self.Mesh`) true)
    (`GameplayStatics.PlaySoundAtLocation` "/Game/Audio/Deaths/Deaths.Deaths" (`self.K2_GetActorLocation`) (struct) 1.0 1.0 0.0 null null null null)
    (`SceneComponent.SetVisibility` (`self.Health Bar Widget`) false false)))

(fn `UserConstructionScript`)